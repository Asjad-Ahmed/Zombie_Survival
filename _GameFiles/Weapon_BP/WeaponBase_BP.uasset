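; Base weapon actor that handles firing effects, projectile spawning and reload animations for its owning character, destroying itself when that character dies.
; BeginPlay gets the character from the Instigator and derives shot interval from fire rate.
; Multi-prefixed events play montages, particles and sound, spawn projectiles and trigger reloads.
; For local players, Tick stretches and aims a laser and dot at the muzzle impact point when the character's DifferentTargets flag is set.
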(event Custom|MULTI_Weapon%20Effects
  (Utilities|FlowControl|Sequence
    (:then_0
      (if (not (Variables|/Game/_GameFiles/Character_Bluprints/Zombie_survival_CharacterBP.Zombie_survival_CharacterBP_C|GetIs%20Crouched? (Variables|Default|GetCharacter%20Ref)))
        (Animation|PlayAnimMontage (Variables|Default|GetCharacter%20Ref) (Variables|Default|GetFire%20Stand%20Animation) 1.0 "None")))
    (:then_1
      (Effects|SpawnEmitterAttached (Variables|Default|GetMuzzleFlash) (Variables|Default|GetSkeletalMesh) "MuzzleFlash" "0, 0, 0" "0, 0, 0" "0.600000,0.600000,0.600000" "SnapToTarget")
      (Audio|PlaySoundatLocation (Variables|Default|GetFiring%20Sound) (Transformation|GetActorLocation) "0, 0, 0" 1.0 1.0 0.0 0 0 0)
      (Effects|SpawnEmitterAttached (Variables|Default|GetAmmoEject) (Variables|Default|GetSkeletalMesh) "AmmoEject" "50.000000, 0, 0" "0, 0, 0" "0.500000,0.500000,0.500000" "SnapToTarget")
      (Niagara|SpawnSystemAttached (Variables|Default|GetMuzzleFlashNiagara) (Variables|Default|GetSkeletalMesh) "MuzzleFlash" "0, 0, 0" "0, 0, 0" "SnapToTarget" true))))

(event Custom|Multi_Weapon_Projectile
  (params (SpawnTransform :type Transform) (Instigator :type Pawn%20Object%20Reference))
  (Game|SpawnActorfromClass (Variables|Default|GetWeaponProjectile) SpawnTransform "AlwaysSpawn" self Instigator))

(event Custom|Multi%20Reload
  (bind _returnvalue (CallFunction|ReloadAnimations))
  (Variables|Default|SetReloadAnimationDelay_0 _returnvalue))

(event EventBeginPlay
  (bind _characterref (Class|CharacterBlueprintInterface|Character(Message) (Variables|Actor|GetInstigator)))
  (Variables|Default|SetCharacter%20Ref _characterref)
  (Variables|Default|SetTimeBetweenShots (/ 6e+01 (Variables|Default|GetWeaponFireRate))))

(event Collision|EventActorBeginOverlap
  (params (OtherActor :type Actor%20Object%20Reference)))

(event EventTick
  (params (DeltaSeconds :type Float%20%28single-precision%29))
  (if (Variables|/Game/_GameFiles/Character_Bluprints/Zombie_survival_CharacterBP.Zombie_survival_CharacterBP_C|GetIsDead? (Variables|Default|GetCharacter%20Ref))
    (Actor|DestroyActor)
    (elif (Pawn|IsLocallyControlled (Variables|Default|GetCharacter%20Ref))
      (|CrosshairGrayOut))))

(fn ConstructionScript)

(fn UseAmmoCondition
  (bind _weapon_current_ammo (Variables|Default|GetWeapon%20Current%20Ammo))
  (bind _returnvalue (<= _weapon_current_ammo 0))
  (if _returnvalue
    (Development|PrintString "NO Ammo")
    (else
      (return _returnvalue))))

(fn ReloadAnimations
  (Components|Animation|PlayAnimation (Variables|Default|GetSkeletalMesh) (Variables|Default|GetReloadingWeapon%20Animation) false)
  (bind _returnvalue (Animation|PlayAnimMontage (Variables|Default|GetCharacter%20Ref) (Variables|Default|GetReloadingPlayer%20Animation) 1.0 "None"))
  (return _returnvalue))

(fn WeaponBase
  (return self))