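; Base projectile for weapons that, on sphere hit, damages players and zombies other than its instigator.
; Message calls identify the target type, then macros sort the hit bone into body, head or limb to scale point damage.
; Flesh hits play blood and sound, then destroy the projectile after a delay; other surfaces get stone impact effects and immediate destruction.
; Unmatched bones on characters trigger nothing, as the default output is unwired.
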(event OnComponentHit(Sphere)
  (params (HitComponent :type Primitive%20Component%20Object%20Reference) (OtherActor :type Actor%20Object%20Reference) (OtherComp :type Primitive%20Component%20Object%20Reference) (NormalImpulse :type Vector :default "0, 0, 0") (Hit :type Hit%20Result%20Structure%20%28by%20ref%29))
  (bind (_bblockinghit _binitialoverlap _time _distance _location _impactpoint _normal _impactnormal _physmat _hitactor _hitcomponent _hitbonename _hititem _faceindex _tracestart) (Collision|BreakHitResult Hit))
  (Variables|Default|SetOther%20Actor OtherActor)
  (Variables|Default|SetHit%20Info "")
  (Variables|Default|SetHitFromDirection _tracestart)
  (Variables|Default|SetHit%20Actor _hitactor)
  (Variables|Default|SetImpactPoint _impactpoint)
  (if (not (== (Variables|Default|GetHit%20Actor) (Variables|Actor|GetInstigator)))
    (Utilities|PlayerIsHit?
      (:true
        (Utilities|DynamicDamage _hitbonename _hitbonename _hitbonename :!label _label
          (:BodyHit
            (CallFunction|ApplyDamage (Variables|Default|GetHit%20Actor) (Variables|Default|GetHitFromDirection) (Variables|Default|GetHit%20Info) (Variables|Default|GetWeapon%20Damage)))
          (:HeadHit
            (CallFunction|ApplyDamage (Variables|Default|GetHit%20Actor) (Variables|Default|GetImpactPoint) (Variables|Default|GetHit%20Info) (* (Variables|Default|GetWeapon%20Damage) 1.6)))
          (:LimbsHit
            (CallFunction|ApplyDamage (Variables|Default|GetHit%20Actor) (Variables|Default|GetImpactPoint) (Variables|Default|GetHit%20Info) (* (Variables|Default|GetWeapon%20Damage) 0.6))))
        (Effects|SpawnEmitteratLocation "/Game/FXVillesBloodVFXPack/Particles/Cascade/Real/P_Blood_BulletHit.P_Blood_BulletHit" (Variables|Default|GetImpactPoint) "0, 0, 0" "2.000000,2.000000,2.000000")
        (Audio|PlaySoundatLocation (Variables|Default|GetSoundHitFlesh) (Variables|Default|GetImpactPoint) "0, 0, 0" 1.0 1.0 0.0 0 0 0)
        (Utilities|FlowControl|Delay 2.0))
      (:false
        (Utilities|ZombieIsHit?
          (:true
            (goto _label))
          (:false
            (Effects|SpawnEmitteratLocation "/Game/MilitaryWeapSilver/FX/P_Impact_Stone_Small_01.P_Impact_Stone_Small_01" (Variables|Default|GetImpactPoint) "0, 0, 0" "2.000000,2.000000,2.000000")
            (Audio|PlaySoundatLocation (Variables|Default|GetSoundHitSurface) (Variables|Default|GetImpactPoint) "0, 0, 0" 1.0 1.0 0.0 0 0 0)))))
    (Actor|DestroyActor)))

(event EventBeginPlay)

(event Collision|EventActorBeginOverlap
  (params (OtherActor :type Actor%20Object%20Reference)))

(event EventTick
  (params (DeltaSeconds :type Float%20%28single-precision%29)))

(fn ConstructionScript)

(fn ApplyDamage
  (params (DamagedActor :type Actor%20Object%20Reference) (HitFromDirection :type Vector%20%28by%20ref%29) (HitInfo :type Hit%20Result%20Structure%20%28by%20ref%29) (BaseDamage :type Float%20%28single-precision%29))
  (Game|Damage|ApplyPointDamage DamagedActor BaseDamage HitFromDirection HitInfo (Game|GetInstigatorController) self "/Script/Engine.DamageType"))