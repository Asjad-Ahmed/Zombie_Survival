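; Multiplayer zombie AI character with randomized or designer-set clothing, built in the construction script, and a random idle pose.
; PawnSensing triggers a closest-player search and AIMoveTo, then a server-to-multicast attack plays one of eight random montages across body and clothing meshes.
; Hand overlaps deal random melee damage to players, gated by DoOnce nodes that a separate multicast event resets.
; Point damage reduces and prints health, with no death handling.
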(event OnSeePawn(PawnSensing)
  (params (Pawn :type Pawn%20Object%20Reference))
  (bind _closestplayer (Variables|Default|GetClosestPlayer))
  (CallFunction|SVRFindPlayerLocation)
  (AI|AIMoveTo self (Transformation|GetWorldLocation (Variables|/Script/Engine.Character|GetMesh _closestplayer)) _closestplayer 45.0 false
    (:OnSuccess
      (CallFunction|SVRZombieAttack))))

(event OnComponentBeginOverlap(R_Hand)
  (params (OverlappedComponent :type Primitive%20Component%20Object%20Reference) (OtherActor :type Actor%20Object%20Reference) (OtherComp :type Primitive%20Component%20Object%20Reference) (OtherBodyIndex :type Integer) (bFromSweep :type Boolean) (SweepResult :type Hit%20Result%20Structure%20%28by%20ref%29))
  ;[1 1 1] Damage Player
  (bind _aszombie_survival_character_bp (Utilities|Casting|CastToZombie_survival_CharacterBP OtherActor))
  (Utilities|FlowControl|DoOnce false
    (:Completed
      (Default|SVRMeleeHit _aszombie_survival_character_bp (Math|Random|RandomFloatinRange 5.0 9.0)))))

(event OnComponentBeginOverlap(L_Hand)
  (params (OverlappedComponent :type Primitive%20Component%20Object%20Reference) (OtherActor :type Actor%20Object%20Reference) (OtherComp :type Primitive%20Component%20Object%20Reference) (OtherBodyIndex :type Integer) (bFromSweep :type Boolean) (SweepResult :type Hit%20Result%20Structure%20%28by%20ref%29))
  ;[1 1 1] Damage Player
  (bind _aszombie_survival_character_bp (Utilities|Casting|CastToZombie_survival_CharacterBP OtherActor))
  (Utilities|FlowControl|DoOnce false
    (:Completed
      (Default|SVRMeleeHit _aszombie_survival_character_bp (Math|Random|RandomFloatinRange 5.0 9.0)))))

(event Custom|SVR_FindPlayerLocation
  (Variables|Default|SetClosestPlayerDistance 2e+03)
  (bind _outactors (Actor|GetAllActorsOfClass "/Game/_GameFiles/Character_Bluprints/Zombie_survival_CharacterBP.Zombie_survival_CharacterBP_C"))
  (for _array_element _outactors
    (if (< (Transformation|GetDistanceTo _array_element self) (Variables|Default|GetClosestPlayerDistance))
      (Variables|Default|SetClosestPlayerDistance (Transformation|GetDistanceTo _array_element self))
      (Variables|Default|SetClosestPlayer _array_element))))

(event Custom|Multi_ZombieAttack
  (if (not (Variables|Default|GetIsAttacking1?))
    (Variables|Default|SetIsAttacking1? true)
    (switch int (Math|Random|RandomIntegerinRange 0 7)
      (:0
        (Animation|Montage|PlayMontage (Variables|Character|GetMesh) "/Game/_Zombie_AI/Animations/Attacks/RArmAtk/Zombie_Atk_1_R_Arm_Montage.Zombie_Atk_1_R_Arm_Montage"
          (:then
            (Animation|Montage|PlayMontage (Variables|Default|Getdenim_shorts_skinned) "/Game/_Zombie_AI/Animations/Attacks/RArmAtk/Zombie_Atk_1_R_Arm_Montage.Zombie_Atk_1_R_Arm_Montage"
              (:then
                (Animation|Montage|PlayMontage (Variables|Default|GetSinglet_Skinned) "/Game/_Zombie_AI/Animations/Attacks/RArmAtk/Zombie_Atk_1_R_Arm_Montage.Zombie_Atk_1_R_Arm_Montage"
                  (:then
                    (Animation|Montage|PlayMontage (Variables|Default|Getpolo_shirt_skinned) "/Game/_Zombie_AI/Animations/Attacks/RArmAtk/Zombie_Atk_1_R_Arm_Montage.Zombie_Atk_1_R_Arm_Montage"))))))
          (:OnCompleted
            (Variables|Default|SetIsAttacking1? false))))
      (:1
        (Animation|Montage|PlayMontage (Variables|Character|GetMesh) "/Game/_Zombie_AI/Animations/Attacks/RArmAtk/Zombie_Atk_2_R_Arm_Montage.Zombie_Atk_2_R_Arm_Montage"
          (:then
            (Animation|Montage|PlayMontage (Variables|Default|Getdenim_shorts_skinned) "/Game/_Zombie_AI/Animations/Attacks/RArmAtk/Zombie_Atk_2_R_Arm_Montage.Zombie_Atk_2_R_Arm_Montage"
              (:then
                (Animation|Montage|PlayMontage (Variables|Default|GetSinglet_Skinned) "/Game/_Zombie_AI/Animations/Attacks/RArmAtk/Zombie_Atk_2_R_Arm_Montage.Zombie_Atk_2_R_Arm_Montage"
                  (:then
                    (Animation|Montage|PlayMontage (Variables|Default|Getpolo_shirt_skinned) "/Game/_Zombie_AI/Animations/Attacks/RArmAtk/Zombie_Atk_2_R_Arm_Montage.Zombie_Atk_2_R_Arm_Montage"))))))
          (:OnCompleted
            (Utilities|FlowControl|Delay 1.0)
            (Variables|Default|SetIsAttacking1? false))))
      (:2
        (Animation|Montage|PlayMontage (Variables|Character|GetMesh) "/Game/_Zombie_AI/Animations/Attacks/RArmAtk/Zombie_Atk_3_R_Arm_Montage.Zombie_Atk_3_R_Arm_Montage"
          (:then
            (Animation|Montage|PlayMontage (Variables|Default|Getdenim_shorts_skinned) "/Game/_Zombie_AI/Animations/Attacks/RArmAtk/Zombie_Atk_3_R_Arm_Montage.Zombie_Atk_3_R_Arm_Montage"
              (:then
                (Animation|Montage|PlayMontage (Variables|Default|GetSinglet_Skinned) "/Game/_Zombie_AI/Animations/Attacks/RArmAtk/Zombie_Atk_3_R_Arm_Montage.Zombie_Atk_3_R_Arm_Montage"
                  (:then
                    (Animation|Montage|PlayMontage (Variables|Default|Getpolo_shirt_skinned) "/Game/_Zombie_AI/Animations/Attacks/RArmAtk/Zombie_Atk_3_R_Arm_Montage.Zombie_Atk_3_R_Arm_Montage"))))))
          (:OnCompleted
            (Utilities|FlowControl|Delay 1.0)
            (Variables|Default|SetIsAttacking1? false))))
      (:3
        (Animation|Montage|PlayMontage (Variables|Character|GetMesh) "/Game/_Zombie_AI/Animations/Attacks/Zombie_Atk_1_BothArms_Montage.Zombie_Atk_1_BothArms_Montage"
          (:then
            (Animation|Montage|PlayMontage (Variables|Default|Getdenim_shorts_skinned) "/Game/_Zombie_AI/Animations/Attacks/Zombie_Atk_1_BothArms_Montage.Zombie_Atk_1_BothArms_Montage"
              (:then
                (Animation|Montage|PlayMontage (Variables|Default|GetSinglet_Skinned) "/Game/_Zombie_AI/Animations/Attacks/Zombie_Atk_1_BothArms_Montage.Zombie_Atk_1_BothArms_Montage"
                  (:then
                    (Animation|Montage|PlayMontage (Variables|Default|Getpolo_shirt_skinned) "/Game/_Zombie_AI/Animations/Attacks/Zombie_Atk_1_BothArms_Montage.Zombie_Atk_1_BothArms_Montage"))))))
          (:OnCompleted
            (Utilities|FlowControl|Delay 1.0)
            (Variables|Default|SetIsAttacking1? false))))
      (:4
        (Animation|Montage|PlayMontage (Variables|Character|GetMesh) "/Game/_Zombie_AI/Animations/Attacks/Zombie_Atk_2_BothArms_Montage.Zombie_Atk_2_BothArms_Montage"
          (:then
            (Animation|Montage|PlayMontage (Variables|Default|Getdenim_shorts_skinned) "/Game/_Zombie_AI/Animations/Attacks/Zombie_Atk_2_BothArms_Montage.Zombie_Atk_2_BothArms_Montage"
              (:then
                (Animation|Montage|PlayMontage (Variables|Default|GetSinglet_Skinned) "/Game/_Zombie_AI/Animations/Attacks/Zombie_Atk_2_BothArms_Montage.Zombie_Atk_2_BothArms_Montage"
                  (:then
                    (Animation|Montage|PlayMontage (Variables|Default|Getpolo_shirt_skinned) "/Game/_Zombie_AI/Animations/Attacks/Zombie_Atk_2_BothArms_Montage.Zombie_Atk_2_BothArms_Montage"))))))
          (:OnCompleted
            (Utilities|FlowControl|Delay 1.0)
            (Variables|Default|SetIsAttacking1? false))))
      (:5
        (Animation|Montage|PlayMontage (Variables|Character|GetMesh) "/Game/_Zombie_AI/Animations/Attacks/LArmAtk/Zombie_Atk_1L_Arm1Montage.Zombie_Atk_1L_Arm1Montage"
          (:then
            (Animation|Montage|PlayMontage (Variables|Default|Getdenim_shorts_skinned) "/Game/_Zombie_AI/Animations/Attacks/LArmAtk/Zombie_Atk_1L_Arm1Montage.Zombie_Atk_1L_Arm1Montage"
              (:then
                (Animation|Montage|PlayMontage (Variables|Default|GetSinglet_Skinned) "/Game/_Zombie_AI/Animations/Attacks/LArmAtk/Zombie_Atk_1L_Arm1Montage.Zombie_Atk_1L_Arm1Montage"
                  (:then
                    (Animation|Montage|PlayMontage (Variables|Default|Getpolo_shirt_skinned) "/Game/_Zombie_AI/Animations/Attacks/LArmAtk/Zombie_Atk_1L_Arm1Montage.Zombie_Atk_1L_Arm1Montage"))))))
          (:OnCompleted
            (Utilities|FlowControl|Delay 1.0)
            (Variables|Default|SetIsAttacking1? false))))
      (:6
        (Animation|Montage|PlayMontage (Variables|Character|GetMesh) "/Game/_Zombie_AI/Animations/Attacks/LArmAtk/Zombie_Atk_2_LArm_Montage.Zombie_Atk_2_LArm_Montage"
          (:then
            (Animation|Montage|PlayMontage (Variables|Default|Getdenim_shorts_skinned) "/Game/_Zombie_AI/Animations/Attacks/LArmAtk/Zombie_Atk_2_LArm_Montage.Zombie_Atk_2_LArm_Montage"
              (:then
                (Animation|Montage|PlayMontage (Variables|Default|GetSinglet_Skinned) "/Game/_Zombie_AI/Animations/Attacks/LArmAtk/Zombie_Atk_2_LArm_Montage.Zombie_Atk_2_LArm_Montage"
                  (:then
                    (Animation|Montage|PlayMontage 0 "/Game/_Zombie_AI/Animations/Attacks/LArmAtk/Zombie_Atk_2_LArm_Montage.Zombie_Atk_2_LArm_Montage"))))))
          (:OnCompleted
            (Utilities|FlowControl|Delay 1.0)
            (Variables|Default|SetIsAttacking1? false))))
      (:7
        (Animation|Montage|PlayMontage (Variables|Character|GetMesh) "/Game/_Zombie_AI/Animations/Attacks/LArmAtk/Zombie_Atk_3_LArm_Montage.Zombie_Atk_3_LArm_Montage"
          (:then
            (Animation|Montage|PlayMontage (Variables|Default|Getdenim_shorts_skinned) "/Game/_Zombie_AI/Animations/Attacks/LArmAtk/Zombie_Atk_3_LArm_Montage.Zombie_Atk_3_LArm_Montage"
              (:then
                (Animation|Montage|PlayMontage (Variables|Default|GetSinglet_Skinned) "/Game/_Zombie_AI/Animations/Attacks/LArmAtk/Zombie_Atk_3_LArm_Montage.Zombie_Atk_3_LArm_Montage"
                  (:then
                    (Animation|Montage|PlayMontage 0 "/Game/_Zombie_AI/Animations/Attacks/LArmAtk/Zombie_Atk_3_LArm_Montage.Zombie_Atk_3_LArm_Montage"))))))
          (:OnCompleted
            (Utilities|FlowControl|Delay 1.0)
            (Variables|Default|SetIsAttacking1? false)))))))

(event Custom|SVR_ResetOnce
  ;[1 1 1] Damage Player
  (CallFunction|MultiResetOnce))

(event Custom|Multi_ResetOnce
  ;[1 1 1] Damage Player
  (Utilities|FlowControl|Sequence
    (:then_0
      (Utilities|FlowControl|DoOnce false) ; enters at Reset
    )
    (:then_1
      (Utilities|FlowControl|DoOnce false) ; enters at Reset
    )))

(event Custom|SVR_ZombieAttack
  (CallFunction|MultiZombieAttack))

(event EventBeginPlay
  (Utilities|FlowControl|Delay 0.3)
  (Utilities|FlowControl|Sequence
    (:then_0
      (Utilities|RandomLocomotionPoses))
    (:then_1
      (Variables|Default|SetCurrentHealth (Variables|Default|GetMaxHealth)))))

(event Game|Damage|EventPointDamage
  (params (Damage :type Float%20%28single-precision%29) (DamageType :type Damage%20Type%20Object%20Reference) (HitLocation :type Vector :default "0, 0, 0") (HitNormal :type Vector :default "0, 0, 0") (HitComponent :type Primitive%20Component%20Object%20Reference) (BoneName :type Name :default "None") (ShotFromDirection :type Vector :default "0, 0, 0") (InstigatedBy :type Controller%20Object%20Reference) (DamageCauser :type Actor%20Object%20Reference) (HitInfo :type Hit%20Result%20Structure%20%28by%20ref%29))
  ;[1 1 1] Take Damage From Bullet
  (bind _output_get (Variables|Default|SetCurrentHealth (- (Variables|Default|GetCurrentHealth) Damage)))
  (Development|PrintString (Utilities|String|ToString(Float) _output_get)))

(fn ConstructionScript
  (bind _material_poloshirt (Variables|Clothing|GetMaterial_PoloShirt))
  (bind _material_singlet (Variables|Clothing|GetMaterial_Singlet))
  (bind _material_beanie (Variables|Clothing|GetMaterial_Beanie))
  (bind _material_shorts (Variables|Clothing|GetMaterial_Shorts))
  (if (Variables|Clothing|GetRandomlyGenerate)
    ;[1 1 1] Hard set random values
    (Variables|Clothing|SetShirtRandomIndex (Math|Random|RandomInteger (LocalVariables|GetShirtOptions)))
    (Variables|Clothing|SetHeadRandomIndex (Math|Random|RandomInteger (LocalVariables|GetHeadOptions)))
    (Variables|Clothing|SetShortsRandomIndex (Math|Random|RandomInteger (LocalVariables|GetShortsOptions)))
    ;[1 1 1] Randomly assign clothing
    (Utilities|FlowControl|Sequence
      (:then_0
        (if (== (Variables|Clothing|GetShirtRandomIndex) 0)
          (Rendering|SetVisibility (Variables|Default|Getpolo_shirt_skinned) false false)
          (Rendering|SetVisibility (Variables|Default|GetSinglet_Skinned) false false)
          (elif (== (Variables|Clothing|GetShirtRandomIndex) 1)
            (Rendering|SetVisibility (Variables|Default|Getpolo_shirt_skinned) true false)
            (Rendering|SetVisibility (Variables|Default|GetSinglet_Skinned) false false)
            (bind _randomindex (CallFunction|RandomMaterialIndexGenerator _material_poloshirt))
            (bind _output_get (Variables|Clothing|SetMaterial_Index_Poloshirt _randomindex))
            (Rendering|Material|SetMaterial (Variables|Default|Getpolo_shirt_skinned) 0 (Utilities|Array|Get(acopy) _material_poloshirt _output_get))
            (elif (== (Variables|Clothing|GetShirtRandomIndex) 2)
              (Rendering|SetVisibility (Variables|Default|GetSinglet_Skinned) true false)
              (Rendering|SetVisibility (Variables|Default|Getpolo_shirt_skinned) false false)
              (bind _randomindex_2 (CallFunction|RandomMaterialIndexGenerator _material_singlet))
              (bind _output_get_2 (Variables|Clothing|SetMaterial_Index_Singlet _randomindex_2))
              (Rendering|Material|SetMaterial (Variables|Default|GetSinglet_Skinned) 0 (Utilities|Array|Get(acopy) _material_singlet _output_get_2))))))
      (:then_1
        (if (== (Variables|Clothing|GetHeadRandomIndex) 0)
          (Rendering|SetVisibility (Variables|Default|Getbeanie_lods) false false)
          (else
            (Rendering|SetVisibility (Variables|Default|Getbeanie_lods) true false)
            (bind _randomindex_3 (CallFunction|RandomMaterialIndexGenerator _material_beanie))
            (bind _output_get_3 (Variables|Clothing|SetMaterial_Index_Beanie _randomindex_3))
            (Rendering|Material|SetMaterial (Variables|Default|Getbeanie_lods) 0 (Utilities|Array|Get(acopy) _material_beanie _output_get_3)))))
      (:then_2
        (if (== (Variables|Clothing|GetShortsRandomIndex) 0)
          (Rendering|SetVisibility (Variables|Default|Getdenim_shorts_skinned) false false)
          (else
            (Rendering|SetVisibility (Variables|Default|Getdenim_shorts_skinned) true false)
            (bind _randomindex_4 (CallFunction|RandomMaterialIndexGenerator _material_shorts))
            (bind _output_get_4 (Variables|Clothing|SetMaterial_Index_Shorts _randomindex_4))
            (Rendering|Material|SetMaterial (Variables|Default|Getdenim_shorts_skinned) 0 (Utilities|Array|Get(acopy) _material_shorts _output_get_4))))))
    (else
      ;[1 1 1] Set clothing based off user input
      (Utilities|FlowControl|Sequence
        (:then_0
          (Rendering|SetVisibility (Variables|Default|Getdenim_shorts_skinned) (Variables|Clothing|GetVisibility_Shorts) false)
          (bind (_materialoutput _materialindexupdated) (CallFunction|IsArrayinBounds (Variables|Clothing|GetMaterial_Shorts) (Variables|Clothing|GetMaterial_Index_Shorts)))
          (Rendering|Material|SetMaterial (Variables|Default|Getdenim_shorts_skinned) 0 _materialoutput)
          (Variables|Clothing|SetMaterial_Index_Shorts _materialindexupdated))
        (:then_1
          (Rendering|SetVisibility (Variables|Default|Getpolo_shirt_skinned) (Variables|Clothing|GetVisibility_Poloshirt) false)
          (bind (_materialoutput_2 _materialindexupdated_2) (CallFunction|IsArrayinBounds (Variables|Clothing|GetMaterial_PoloShirt) (Variables|Clothing|GetMaterial_Index_Poloshirt)))
          (Rendering|Material|SetMaterial (Variables|Default|Getpolo_shirt_skinned) 0 _materialoutput_2)
          (Variables|Clothing|SetMaterial_Index_Poloshirt _materialindexupdated_2))
        (:then_2
          (Rendering|SetVisibility (Variables|Default|GetSinglet_Skinned) (Variables|Clothing|GetVisibility_Singlet) false)
          (bind (_materialoutput_3 _materialindexupdated_3) (CallFunction|IsArrayinBounds (Variables|Clothing|GetMaterial_Singlet) (Variables|Clothing|GetMaterial_Index_Singlet)))
          (Rendering|Material|SetMaterial (Variables|Default|GetSinglet_Skinned) 0 _materialoutput_3)
          (Variables|Clothing|SetMaterial_Index_Singlet _materialindexupdated_3))
        (:then_3
          (Rendering|SetVisibility (Variables|Default|Getbeanie_lods) (Variables|Clothing|GetVisibility_Singlet) false)
          (bind (_materialoutput_4 _materialindexupdated_4) (CallFunction|IsArrayinBounds (Variables|Clothing|GetMaterial_Beanie) (Variables|Clothing|GetMaterial_Index_Beanie)))
          (Rendering|Material|SetMaterial (Variables|Default|Getbeanie_lods) 0 _materialoutput_4)
          (Variables|Clothing|SetMaterial_Index_Beanie _materialindexupdated_4))))))

(fn RandomMaterialIndexGenerator
  (params (MaterialArray :type Array%20of%20Material%20Instance%20Object%20References))
  (return (Math|Random|RandomInteger (Utilities|Array|Length MaterialArray))))

(fn IsArrayinBounds
  (params (MaterialArray :type Array%20of%20Material%20Instance%20Object%20References) (MaterialIndex :type Integer))
  (bind _returnvalue (Utilities|Array|Length MaterialArray))
  (bind _returnvalue_2 (- _returnvalue 1))
  (if (> (+ MaterialIndex 1) (Utilities|Array|Length MaterialArray))
    (return (Utilities|Array|Get(acopy) MaterialArray _returnvalue_2) _returnvalue_2)
    (else
      (return (Utilities|Array|Get(acopy) MaterialArray MaterialIndex) MaterialIndex))))

(fn WhichMontagePlaying?
  (params (Montage :type Anim%20Montage%20Object%20Reference))
  (return (Animation|Montage|MontageIsPlaying (Components|SkeletalMesh|GetAnimInstance (Variables|Character|GetMesh)) Montage)))

(fn StopAttackingMontage
  (params (Montage :type Anim%20Montage%20Object%20Reference) (Montage1 :type Anim%20Montage%20Object%20Reference) (Montage2 :type Anim%20Montage%20Object%20Reference) (Montage3 :type Anim%20Montage%20Object%20Reference))
  (bind _mesh (Variables|Character|GetMesh))
  (bind _returnvalue (Components|SkeletalMesh|GetAnimInstance _mesh))
  (Animation|Montage|MontageStop _returnvalue 0.3 Montage)
  (Animation|Montage|MontageStop _returnvalue 0.3 Montage1)
  (Animation|Montage|MontageStop _returnvalue 0.3 Montage2)
  (Animation|Montage|MontageStop _returnvalue 0.3 Montage3)
  (return))

(fn ZombieRef
  (return self))